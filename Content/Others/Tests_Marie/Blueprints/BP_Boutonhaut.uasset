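; BP_Boutonhaut is a clickable button actor that toggles the upward gesture selection.
; On click, it switches off the down button (BP_Boutonbas) or else the face button (BP_Boutonface) if either is active, otherwise calling Childisclicked.
; It then flips its own state, mirrors it to Hautclicked alongside a BP_Geste lookup, and swaps the cube's on/off material.
; Decliquerhaut lets other gesture buttons switch it off, keeping selection exclusive.
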(event `self.ReceiveActorOnClicked`
  (params (ButtonPressed :type "Key Structure"))
  ; Ce qui se passe quand on clique sur le bouton geste vers le haut
  (bind _returnvalue (`GameplayStatics.GetActorOfClass` "/Game/Others/Tests_Marie/Blueprints/BP_Boutonbas.BP_Boutonbas_C"))
  (if (`/Game/Others/Tests_Marie/Blueprints/BP_Boutonbas.Boutonbasisclicked` _returnvalue)
    (bind _returnvalue_2 (`GameplayStatics.GetActorOfClass` "/Game/Others/Tests_Marie/Blueprints/BP_Boutonbas.BP_Boutonbas_C"))
    (`/Game/Others/Tests_Marie/Blueprints/BP_Boutonbas.Decliquerbas` _returnvalue_2)
    (else
      (bind _returnvalue_3 (`GameplayStatics.GetActorOfClass` "/Game/Others/Tests_Marie/Blueprints/BP_Boutonface.BP_Boutonface_C"))
      (if (`/Game/Others/Tests_Marie/Blueprints/BP_Boutonface.Boutonversfaceisclicked` _returnvalue_3)
        (bind _returnvalue_4 (`GameplayStatics.GetActorOfClass` "/Game/Others/Tests_Marie/Blueprints/BP_Boutonface.BP_Boutonface_C"))
        (`/Game/Others/Tests_Marie/Blueprints/BP_Boutonface.Decliquerface` _returnvalue_4)
        (else
          (`self.Childisclicked`)))))
  (if (`self.Boutonenhautisclicked`)
    (set `self.Boutonenhautisclicked` false)
    (`GameplayStatics.GetActorOfClass` "/Game/Others/Tests_Marie/Blueprints/BP_Geste.BP_Geste_C")
    (set `self.hautclicked` false)
    (`PrimitiveComponent.SetMaterial` (`self.Cube`) 0 "/Game/Others/Tests_Marie/Matériaux/M_Bouton_haut_off.M_Bouton_haut_off")
    (else
      (set `self.Boutonenhautisclicked` true)
      (`GameplayStatics.GetActorOfClass` "/Game/Others/Tests_Marie/Blueprints/BP_Geste.BP_Geste_C")
      (set `self.hautclicked` true)
      (`PrimitiveComponent.SetMaterial` (`self.Cube`) 0 "/Game/Others/Tests_Marie/Matériaux/M_Bouton_haut_on.M_Bouton_haut_on"))))

(event `Decliquerhaut`
  ; Décliquer haut : événement permettant de passer le bouton geste vers le haut en off si un autre bouton geste est cliqué
  (set `self.Boutonenhautisclicked` false)
  (set `self.hautclicked` false)
  (`PrimitiveComponent.SetMaterial` (`self.Cube`) 0 "/Game/Others/Tests_Marie/Matériaux/M_Bouton_haut_off.M_Bouton_haut_off"))

(fn `UserConstructionScript`
  (`parent.UserConstructionScript`))