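; BP_validation is a clickable validation button actor that becomes usable only when both the gesture and lever indicator lights are on.
; Every tick it looks up BP_Voyant_geste and BP_Voyant_levier by class and sets Isactive to false if either reports being off.
; A click while Isactive is true changes its TextRender label to "Validé".
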(event `self.ReceiveTick`
  (params (DeltaSeconds :type "Float (single-precision)"))
  ; Vérifie si les deux voyants sont allumés et si oui, active la possibilité de valider
  (bind _returnvalue (`GameplayStatics.GetActorOfClass` "/Game/Others/Tests_Marie/Blueprints/BP_Voyant_geste.BP_Voyant_geste_C"))
  (bind _returnvalue_2 (`GameplayStatics.GetActorOfClass` "/Game/Others/Tests_Marie/Blueprints/BP_Voyant_levier.BP_Voyant_levier_C"))
  (if (`/Game/Others/Tests_Marie/Blueprints/BP_Voyant_levier.Esteteintlevier` _returnvalue_2)
    (set `self.Isactive` false :!label _label)
    (elif (`/Game/Others/Tests_Marie/Blueprints/BP_Voyant_geste.Esteteint` _returnvalue)
      (goto _label)
      (else
        (set `self.Isactive` true)))))

(event `self.ReceiveActorOnClicked`
  (params (ButtonPressed :type "Key Structure"))
  ; Au clic, change le texte du bouton s'il est actif
  (if (`self.Isactive`)
    (`TextRenderComponent.K2_SetText` (`self.TextRender`) (`self.Validé`))))

(fn `UserConstructionScript`)