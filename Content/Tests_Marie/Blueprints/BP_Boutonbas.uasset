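; BP_Boutonbas is a clickable button actor that toggles the downward gesture option on and off.
; A click first switches off an active face or up button through GetActorOfClass lookups, or calls Childisclicked if neither is active.
; It then flips its own clicked state, the Basclicked gesture flag and the cube's on/off material.
; The Decliquerbas event lets another gesture button switch this one off, keeping the selection exclusive.
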(event `self.ReceiveActorOnClicked`
  (params (ButtonPressed :type "Key Structure"))
  ; Ce qui se passe quand on clique sur le bouton geste vers le bas
  (bind _returnvalue (`GameplayStatics.GetActorOfClass` "/Game/Tests_Marie/Blueprints/BP_Boutonface.BP_Boutonface_C"))
  (if (`/Game/Tests_Marie/Blueprints/BP_Boutonface.Boutonversfaceisclicked` _returnvalue)
    (bind _returnvalue_2 (`GameplayStatics.GetActorOfClass` "/Game/Tests_Marie/Blueprints/BP_Boutonface.BP_Boutonface_C"))
    (`/Game/Tests_Marie/Blueprints/BP_Boutonface.Decliquerface` _returnvalue_2)
    (else
      (bind _returnvalue_3 (`GameplayStatics.GetActorOfClass` "/Game/Tests_Marie/Blueprints/BP_Boutonhaut.BP_Boutonhaut_C"))
      (if (`/Game/Tests_Marie/Blueprints/BP_Boutonhaut.Boutonenhautisclicked` _returnvalue_3)
        (bind _returnvalue_4 (`GameplayStatics.GetActorOfClass` "/Game/Tests_Marie/Blueprints/BP_Boutonhaut.BP_Boutonhaut_C"))
        (`/Game/Tests_Marie/Blueprints/BP_Boutonhaut.Decliquerhaut` _returnvalue_4)
        (else
          (`self.Childisclicked`)))))
  (if (`self.Boutonbasisclicked`)
    (set `self.Boutonbasisclicked` false)
    (`GameplayStatics.GetActorOfClass` "/Game/Tests_Marie/Blueprints/BP_Geste.BP_Geste_C")
    (set `self.basclicked` false)
    (`PrimitiveComponent.SetMaterial` (`self.Cube`) 0 "/Game/Tests_Marie/Matériaux/M_Bouton_bas_off.M_Bouton_bas_off")
    (else
      (set `self.Boutonbasisclicked` true)
      (`GameplayStatics.GetActorOfClass` "/Game/Tests_Marie/Blueprints/BP_Geste.BP_Geste_C")
      (set `self.basclicked` true)
      (`PrimitiveComponent.SetMaterial` (`self.Cube`) 0 "/Game/Tests_Marie/Matériaux/M_Bouton_bas_on.M_Bouton_bas_on"))))

(event `Decliquerbas`
  ; Décliquer bas : événement permettant de passer le bouton geste vers le bas en off si un autre bouton geste est cliqué
  (set `self.Boutonbasisclicked` false)
  (set `self.basclicked` false)
  (`PrimitiveComponent.SetMaterial` (`self.Cube`) 0 "/Game/Tests_Marie/Matériaux/M_Bouton_bas_off.M_Bouton_bas_off"))

(fn `UserConstructionScript`
  (`parent.UserConstructionScript`))