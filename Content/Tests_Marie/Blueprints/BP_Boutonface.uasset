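; BP_Boutonface is a clickable button actor that toggles the "gesture toward face" option, in what appears to be a set of gesture buttons.
; On click it switches off an active BP_Boutonbas or BP_Boutonhaut, or calls Childisclicked if neither is active.
; It then flips its state, the Faceclicked flag linked to BP_Geste and the Cube's on/off material.
; Decliquerface provides an event to force it off.
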(event `self.ReceiveActorOnClicked`
  (params (ButtonPressed :type "Key Structure"))
  ; Ce qui se passe quand on clique sur le bouton gestz vers face
  (bind _returnvalue (`GameplayStatics.GetActorOfClass` "/Game/Tests_Marie/Blueprints/BP_Boutonbas.BP_Boutonbas_C"))
  (if (`/Game/Tests_Marie/Blueprints/BP_Boutonbas.Boutonbasisclicked` _returnvalue)
    (bind _returnvalue_2 (`GameplayStatics.GetActorOfClass` "/Game/Tests_Marie/Blueprints/BP_Boutonbas.BP_Boutonbas_C"))
    (`/Game/Tests_Marie/Blueprints/BP_Boutonbas.Decliquerbas` _returnvalue_2)
    (else
      (bind _returnvalue_3 (`GameplayStatics.GetActorOfClass` "/Game/Tests_Marie/Blueprints/BP_Boutonhaut.BP_Boutonhaut_C"))
      (if (`/Game/Tests_Marie/Blueprints/BP_Boutonhaut.Boutonenhautisclicked` _returnvalue_3)
        (bind _returnvalue_4 (`GameplayStatics.GetActorOfClass` "/Game/Tests_Marie/Blueprints/BP_Boutonhaut.BP_Boutonhaut_C"))
        (`/Game/Tests_Marie/Blueprints/BP_Boutonhaut.Decliquerhaut` _returnvalue_4)
        (else
          (`self.Childisclicked`)))))
  (if (`self.Boutonversfaceisclicked`)
    (set `self.Boutonversfaceisclicked` false)
    (`GameplayStatics.GetActorOfClass` "/Game/Tests_Marie/Blueprints/BP_Geste.BP_Geste_C")
    (set `self.faceclicked` false)
    (`PrimitiveComponent.SetMaterial` (`self.Cube`) 0 "/Game/Tests_Marie/Matériaux/M_Bouton_face_off.M_Bouton_face_off")
    (else
      (set `self.Boutonversfaceisclicked` true)
      (`GameplayStatics.GetActorOfClass` "/Game/Tests_Marie/Blueprints/BP_Geste.BP_Geste_C")
      (set `self.faceclicked` true)
      (`PrimitiveComponent.SetMaterial` (`self.Cube`) 0 "/Game/Tests_Marie/Matériaux/M_Bouton_face_on.M_Bouton_face_on"))))

(event `Decliquerface`
  ; Décliquer face : événement permettant de passer le bouton geste vers face en off si un autre bouton geste est cliqué
  (set `self.Boutonversfaceisclicked` false)
  (set `self.faceclicked` false)
  (`PrimitiveComponent.SetMaterial` (`self.Cube`) 0 "/Game/Tests_Marie/Matériaux/M_Bouton_face_off.M_Bouton_face_off"))

(fn `UserConstructionScript`
  (`parent.UserConstructionScript`))