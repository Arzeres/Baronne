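; BP_Levier is a clickable lever that moves through two intermediate notches between its top and bottom positions, reversing direction at each end.
; Each click rotates pitch by 20 degrees, with limit checks setting the end-reached and direction booleans for the next click.
; It also drives BP_Voyant_levier, clearing that indicator's off flag on every click and setting it when pitch reaches the upper limit.
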(event `self.ReceiveActorOnClicked`
  (params (ButtonPressed :type "Key Structure"))
  (bind _pitch (.pitch (`self.K2_GetActorRotation`)))
  ; Système qui fait monter le levier jusqu'en haut, puis descendre jusqu'en bas, avec les deux crans intermédiaires. Envoie également les informations au voyant levier pour gérer l'allumage
  (bind _returnvalue (`GameplayStatics.GetActorOfClass` "/Game/Tests_Marie/Blueprints/BP_Voyant_levier.BP_Voyant_levier_C"))
  (set `/Game/Tests_Marie/Blueprints/BP_Voyant_levier.Esteteintlevier` false _returnvalue)
  (if (`self.20atteint`)
    (set `self.Onmonte` false)
    (`self.K2_AddActorLocalRotation` (struct :`Pitch` 20.0) :!label _label)
    (set `self.20atteint` false)
    (`/Engine/EditorBlueprintResources/StandardMacros.CompareFloat` _pitch 79.0
      (:`>`
        _)
      (:`==`
        _))
    (set `self.80atteint` true)
    (set `self.Onmonte` true)
    (bind _returnvalue_2 (`GameplayStatics.GetActorOfClass` "/Game/Tests_Marie/Blueprints/BP_Voyant_levier.BP_Voyant_levier_C"))
    (set `/Game/Tests_Marie/Blueprints/BP_Voyant_levier.Esteteintlevier` true _returnvalue_2)
    (else
      (if (`self.Onmonte`)
        _
        (elif (`self.80atteint`)
          _
          (else
            (goto _label))))
      (`self.K2_AddActorLocalRotation` (struct :`Pitch` -20.0))
      (set `self.80atteint` false)
      (`/Engine/EditorBlueprintResources/StandardMacros.CompareFloat` _pitch 21.0
        (:`==`
          _)
        (:`<`
          _))
      (set `self.20atteint` true))))

(fn `UserConstructionScript`)