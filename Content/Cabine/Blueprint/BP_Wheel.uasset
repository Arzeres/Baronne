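; BP_Wheel is a clickable washing-machine knob (Boutonlavelinge) that selects one of four EmotionIndex states.
; Each actor click advances the index, wrapping from 3 to 0, and plays the Rotation timeline, which adds interpolated local yaw every update.
; The knob's click event switches the level's BP_LED_Wheel on for indices 1 and 2, off otherwise.
; ResetWheel restores index, knob rotation and LED.
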(event `self.ReceiveBeginPlay`
  (bind _returnvalue (`GameplayStatics.GetActorOfClass` "/Game/Cabine/Blueprint/BP_LED_Wheel.BP_LED_Wheel_C"))
  (set `self.refLedWheel` _returnvalue))

(event `self.ReceiveActorOnClicked`
  (params (ButtonPressed :type "Key Structure"))
  (bind _emotionindex (`self.emotionIndex`))
  ; Rotate the wheel and set the index
  (`/Engine/EditorBlueprintResources/StandardMacros.CompareInt` _emotionindex 3
    (:`==`
      (set `self.emotionIndex` 0)
      (bind (_direction _newtrack_0) (`Timeline|rotation` :!via `PlayFromStart` :!label _label)
        (:`Update`
          (`SceneComponent.K2_AddLocalRotation` (`self.boutonlavelinge`) (`KismetMathLibrary.MakeRotator` 0.0 0.0 (`KismetMathLibrary.Lerp` 0.0 90.0 _newtrack_0)) false false))))
    (:`<`
      (bind _result (`/Engine/EditorBlueprintResources/StandardMacros.IncrementInt` _emotionindex)
        (:`  `
          (set `self.emotionIndex` _result)
          (goto _label :!via `PlayFromStart`))))))

(event `self.boutonlavelinge.OnClicked`
  (params (TouchedComponent :type "PrimitiveComponent Object Reference") (ButtonPressed :type "Key Structure"))
  ; if index == 1
  (if (== (`self.emotionIndex`) 1)
    (`/Game/Cabine/Blueprint/BP_LED.SwitchOn` (`self.refLedWheel`))
    (else
      ; if index == 2
      (if (== (`self.emotionIndex`) 2)
        (`/Game/Cabine/Blueprint/BP_LED.SwitchOn` (`self.refLedWheel`))
        (else
          (`/Game/Cabine/Blueprint/BP_LED.SwitchOff` (`self.refLedWheel`)))))))

(fn `Reset Wheel`
  (set `self.emotionIndex` 0)
  (`SceneComponent.K2_SetRelativeRotation` (`self.boutonlavelinge`) (struct :`Pitch` 30.0) false false)
  (`/Game/Cabine/Blueprint/BP_LED.SwitchOff` (`self.refLedWheel`)))

(fn `UserConstructionScript`)