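; Clickable cabin lever that steps back and forth through three positions (0, 1, 2, 1, 0), ignoring clicks while moving.
; Each click updates the index, plays a sound and uses a timeline to interpolate the lever's pitch between angles.
; The index change switches the BP_LEDLevers light off at zero and on otherwise, and OnPositionUpdate fires when movement ends.
; ResetLever restores index zero and switches the LED off.
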(event `self.ReceiveActorOnClicked`
  (params (ButtonPressed :type "Key Structure"))
  ; If the lever is already moving the player can't trigger it
  (if (not (`self.IsMoving`))
    (`self.PositionIndex`)
    (set `self.IsMoving` true)
    (`GameplayStatics.SpawnSound2D` "/Game/Others/Tests_Marie/Sons/levier.levier" 1.0 1.0 0.0 null)
    (bind (_direction _lever) (`Timeline|Timeline_1` :!via `PlayFromStart`)
      (:`Update`
        (`SceneComponent.K2_SetRelativeRotation` (`self.Lever`) (`KismetMathLibrary.MakeRotator` 0.0 (`KismetMathLibrary.Lerp` (`self.StartAngle`) (`self.EndAngle`) _lever)) false false))
      (:`Finished`
        (set `self.IsMoving` false)
        (`self.OnPositionUpdate`)))))

(event `self.ReceiveBeginPlay`
  (bind _returnvalue (`GameplayStatics.GetActorOfClass` "/Game/Cabine/Blueprint/BP_LEDLevers.BP_LEDLevers_C"))
  (set `self.BPLedLeversRef` _returnvalue))

(fn `PositionIndex`
  ; Change the position and the number of the index
  (set `self.StartAngle` (* (`self.Angle`) (`self.IndexPosition`)))
  (if (`self.Reverse`)
    (bind _output_get (set `self.IndexPosition` (+ (`self.IndexPosition`) -1)))
    (if (== _output_get 0)
      (`/Game/Cabine/Blueprint/BP_LED.SwitchOff` (`self.BPLedLeversRef`))
      (set `self.Reverse` false)
      (else
        (`/Game/Cabine/Blueprint/BP_LED.SwitchOn` (`self.BPLedLeversRef`) :!label _label)
        (if (== (stale _output_get_2) 2)
          (set `self.Reverse` true))))
    (else
      (bind _output_get_2 (set `self.IndexPosition` (+ (`self.IndexPosition`) 1)))
      (goto _label)))
  (set `self.EndAngle` (* (`self.Angle`) (`self.IndexPosition`))))

(fn `ResetLever`
  (set `self.IndexPosition` 0)
  (set `self.Reverse` false)
  (`SceneComponent.K2_SetRelativeLocationAndRotation` :`self` (`self.Lever`))
  (`/Game/Cabine/Blueprint/BP_LED.SwitchOff` (`self.BPLedLeversRef`)))

(fn `UserConstructionScript`
  (`SceneComponent.K2_SetRelativeRotation` (`self.DefaultSceneRoot`) (`KismetMathLibrary.MakeRotator` 0.0 (`self.StartAngle`)) false false))