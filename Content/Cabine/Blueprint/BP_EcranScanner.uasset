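; BP_EcranScanner is a scanner screen that switches material and reveals scanner text when an NPC is allowed to arrive.
; It caches BP_CrystalBall on BeginPlay and polls its PNJpeutarriver flag every Tick, updating the display after a short delay.
; ResetEcranScanner swaps to another material and hides both the scanner text and the comfort text actors, which are found by class lookup.
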(event `self.ReceiveBeginPlay`
  (bind _returnvalue (`GameplayStatics.GetActorOfClass` "/Game/Cabine/Blueprint/BP_CrystalBall.BP_CrystalBall_C"))
  (set `self.BPcrystalballref` _returnvalue))

(event `self.ReceiveTick`
  (params (DeltaSeconds :type "Float (single-precision)"))
  (if (`/Game/Cabine/Blueprint/BP_CrystalBall.PNJpeutarriver` (`self.BPcrystalballref`))
    (`KismetSystemLibrary.Delay` 3.0)
    (`PrimitiveComponent.SetMaterial` (`self.EcranScanner`) 0 "/Game/Cabine/Materials/Material_005.Material_005")
    (bind _returnvalue (`GameplayStatics.GetActorOfClass` "/Game/Cabine/Blueprint/BP_textescanner.BP_textescanner_C"))
    (`SceneComponent.SetVisibility` (`Actor.RootComponent` _returnvalue) true false)))

(fn `ResetEcranScanner`
  (`PrimitiveComponent.SetMaterial` (`self.EcranScanner`) 0 "/Game/Cabine/Meshes/CabineExt/Material_013.Material_013")
  (bind _returnvalue (`GameplayStatics.GetActorOfClass` "/Game/Cabine/Blueprint/BP_textescanner.BP_textescanner_C"))
  (`SceneComponent.SetVisibility` (`Actor.RootComponent` _returnvalue) false false)
  (bind _returnvalue_2 (`GameplayStatics.GetActorOfClass` "/Game/Cabine/Blueprint/BP_textescannerreconfort.BP_textescannerreconfort_C"))
  (`SceneComponent.SetVisibility` (`Actor.RootComponent` _returnvalue_2) false false))

(fn `UserConstructionScript`)