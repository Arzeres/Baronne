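; Cabin control panel with clickable ATM buttons and a pendulum pull that confirms the player's choice.
; A first click zooms to the ATM camera; pressing top or middle then releases the other, lights the ATM LED and blends back to the player.
; The bottom button and Pannophrases only zoom in.
; When validation is allowed and its LED is on, the pendulum drops and the view moves to the animatronic, then exterior cabin camera.
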(event `self.ReceiveBeginPlay`
  ; Get refs
  (bind _returnvalue (`GameplayStatics.GetActorOfClass` "/Game/Cabine/Blueprint/BP_LED_ATM.BP_LED_ATM_C"))
  (set `self.LEDATMref` _returnvalue)
  (bind _returnvalue_2 (`GameplayStatics.GetActorOfClass` "/Game/Cabine/Blueprint/BP_LeverHead.BP_LeverHead_C"))
  (set `self.HeadLeverRef` _returnvalue_2)
  (bind _returnvalue_3 (`GameplayStatics.GetActorOfClass` "/Game/Camera/BP_Zoom_ATM.BP_Zoom_ATM_C"))
  (set `self.CamZoomATMRef` _returnvalue_3)
  (bind _returnvalue_4 (`GameplayStatics.GetActorOfClass` "/Game/FirstPerson/Blueprints/BP_FirstPersonCharacter.BP_FirstPersonCharacter_C"))
  (set `self.Playercamref` _returnvalue_4)
  (bind _returnvalue_5 (`GameplayStatics.GetActorOfClass` "/Game/Cabine/Blueprint/BP_LEDValidation.BP_LEDValidation_C"))
  (set `self.LEDvalidationref` _returnvalue_5)
  (bind _returnvalue_6 (`GameplayStatics.GetActorOfClass` "/Game/Camera/BP_CameraAnimatronique.BP_CameraAnimatronique_C"))
  (set `self.CamAnimatroniqueref` _returnvalue_6)
  (bind _returnvalue_7 (`GameplayStatics.GetActorOfClass` "/Game/Camera/BP_CabineExtZoom.BP_CabineExtZoom_C"))
  (set `self.CabineExtZoomRef` _returnvalue_7))

(event `self.TopButtonATM.OnClicked`
  (params (TouchedComponent :type "PrimitiveComponent Object Reference") (ButtonPressed :type "Key Structure"))
  (bind _returnvalue (`GameplayStatics.GetPlayerController` 0))
  (bind _topbuttonatm (`self.TopButtonATM`))
  (bind _topbuttonatm_2 (`self.TopButtonATM`))
  ; Enfonce et relève le bouton
  ; ATM top button on zoomed view
  (if (`self.IsATMZoomed`)
    (if (`self.IsMiddleButtonPressed`)
      (`SceneComponent.K2_AddLocalOffset` (`self.MiddleButtonATM`) (0.0 0.0 1.0) false false)
      (set `self.IsMiddleButtonPressed` false)
      (`SceneComponent.K2_AddLocalOffset` _topbuttonatm (0.0 0.0 -1.0) false false :!label _label)
      (`PrimitiveComponent.SetMaterial` _topbuttonatm_2 0 "/Game/Cabine/Materials/Boutonpresse.Boutonpresse")
      (set `self.IsTopButtonPressed` true)
      ; ATM top button on player view
      (`/Game/Cabine/Blueprint/BP_LED.SwitchOn` (`self.LEDATMref`))
      (set `self.IsATMZoomed` false)
      (`PlayerController.SetViewTargetWithBlend` _returnvalue (`self.Playercamref`) 0.75 "VTBlend_Linear" 0.0 false)
      (elif (`self.IsTopButtonPressed`)
        (`SceneComponent.K2_AddLocalOffset` _topbuttonatm (0.0 0.0 1.0) false false)
        (`PrimitiveComponent.SetMaterial` _topbuttonatm_2 0 "/Game/Cabine/Materials/Boutonpaspresse.Boutonpaspresse")
        (set `self.IsTopButtonPressed` false)
        (`/Game/Cabine/Blueprint/BP_LED.SwitchOff` (`self.LEDATMref`))
        (else
          (goto _label))))
    (else
      (`PlayerController.SetViewTargetWithBlend` _returnvalue (`self.CamZoomATMRef`) 0.75 "VTBlend_Linear" 0.0 false)
      (set `self.IsATMZoomed` true))))

(event `self.MiddleButtonATM.OnClicked`
  (params (TouchedComponent :type "PrimitiveComponent Object Reference") (ButtonPressed :type "Key Structure"))
  (bind _returnvalue (`GameplayStatics.GetPlayerController` 0))
  (bind _middlebuttonatm (`self.MiddleButtonATM`))
  ; ATM middle button on zommed view
  (if (`self.IsATMZoomed`)
    ; Enfonce et relève le bouton
    (if (`self.IsTopButtonPressed`)
      (`SceneComponent.K2_AddLocalOffset` (`self.TopButtonATM`) (0.0 0.0 1.0) false false)
      (set `self.IsTopButtonPressed` false)
      (`SceneComponent.K2_AddLocalOffset` _middlebuttonatm (0.0 0.0 -1.0) false false :!label _label_2)
      (set `self.IsMiddleButtonPressed` true)
      ; ATM middle button on player s view
      (`/Game/Cabine/Blueprint/BP_LED.SwitchOn` (`self.LEDATMref`))
      (set `self.IsATMZoomed` false)
      (`PlayerController.SetViewTargetWithBlend` _returnvalue (`self.Playercamref`) 0.75 "VTBlend_Linear" 0.0 false)
      (elif (`self.IsMiddleButtonPressed`)
        (`SceneComponent.K2_AddLocalOffset` _middlebuttonatm (0.0 0.0 1.0) false false)
        (set `self.IsMiddleButtonPressed` false)
        (`/Game/Cabine/Blueprint/BP_LED.SwitchOff` (`self.LEDATMref`))
        (else
          (goto _label_2))))
    (else
      (`PlayerController.SetViewTargetWithBlend` _returnvalue (`self.CamZoomATMRef`) 0.75 "VTBlend_Linear" 0.0 false)
      (set `self.IsATMZoomed` true))))

(event `self.BottomButtonATM.OnClicked`
  (params (TouchedComponent :type "PrimitiveComponent Object Reference") (ButtonPressed :type "Key Structure"))
  ; ATM bottom button on zommed view
  (if (not (`self.IsATMZoomed`)) :!label _label_3
    (`PlayerController.SetViewTargetWithBlend` (`GameplayStatics.GetPlayerController` 0) (`self.CamZoomATMRef`) 0.75 "VTBlend_Linear" 0.0 false)
    (set `self.IsATMZoomed` true)))

(event `self.panno-phrases.OnClicked`
  (params (TouchedComponent :type "PrimitiveComponent Object Reference") (ButtonPressed :type "Key Structure"))
  (goto _label_3))

(event `self.Pendule.OnClicked`
  (params (TouchedComponent :type "PrimitiveComponent Object Reference") (ButtonPressed :type "Key Structure"))
  (if (`self.Peutetrevalide`)
    (if (not (`/Game/Cabine/Blueprint/BP_LED.isOff` (`self.LEDvalidationref`)))
      (`SceneComponent.K2_AddLocalOffset` (`self.chaine`) (0.0 0.0 -30.0) false false)
      (`SceneComponent.K2_AddLocalOffset` (`self.Pendule`) (0.0 0.0 -30.0) false false)
      (`KismetSystemLibrary.Delay` 0.5)
      (`PlayerController.SetViewTargetWithBlend` (`GameplayStatics.GetPlayerController` 0) (`self.CamAnimatroniqueref`) 0.75 "VTBlend_Linear" 0.0 false)
      (`KismetSystemLibrary.Delay` 2.0)
      (`PlayerController.SetViewTargetWithBlend` (`GameplayStatics.GetPlayerController` 0) (`self.CabineExtZoomRef`) 0.75 "VTBlend_Linear" 0.0 false))))

(fn `NewFunction`)

(fn `UserConstructionScript`)