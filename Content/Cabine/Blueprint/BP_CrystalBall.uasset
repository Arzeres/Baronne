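; BP_CrystalBall is a cabin prop that shows a client-specific material on its PlaceholderEdouard component while PNJpeutarriver (NPC can arrive) is true.
; Every Tick it looks up BP_ControlPanel and switches on its Listeclients value to pick the Eliza, Edouard or Camille material, with the last two cases sharing Camille.
; When the flag is false, it applies M_Basic_Wall instead.
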(event `self.ReceiveTick`
  (params (DeltaSeconds :type "Float (single-precision)"))
  (if (`self.PNJpeutarriver`)
    (bind _returnvalue (`GameplayStatics.GetActorOfClass` "/Game/Cabine/Blueprint/BP_ControlPanel.BP_ControlPanel_C"))
    (set `self.BPcontrolpanelref` _returnvalue)
    (switch `/Game/PNJ/Listeclients` (`/Game/Cabine/Blueprint/BP_ControlPanel.Listeclients` (`self.BPcontrolpanelref`))
      (:`NewEnumerator0`
        (`PrimitiveComponent.SetMaterial` (`self.Placeholder-Edouard`) 0 "/Game/PNJ/M-Eliza_Inst.M-Eliza_Inst"))
      (:`NewEnumerator1`
        (`PrimitiveComponent.SetMaterial` (`self.Placeholder-Edouard`) 0 "/Game/PNJ/M-Edouard_Inst.M-Edouard_Inst"))
      (:`NewEnumerator2`
        (`PrimitiveComponent.SetMaterial` (`self.Placeholder-Edouard`) 0 "/Game/PNJ/M_Camille_Inst.M_Camille_Inst" :!label _label))
      (:`NewEnumerator3`
        (goto _label)))
    (else
      (`PrimitiveComponent.SetMaterial` (`self.Placeholder-Edouard`) 0 "/Game/Others/StarterContent/Materials/M_Basic_Wall.M_Basic_Wall"))))

(fn `UserConstructionScript`)