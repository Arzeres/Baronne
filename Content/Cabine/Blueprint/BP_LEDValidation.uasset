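; BP_LEDValidation is a validation LED in the cabin that lights up when the ATM, wheel and lever checks all pass.
; BeginPlay caches those three LEDs and the control panel by class lookup.
; Every Tick, it calls the parent's SwitchOn if the panel's Peutetrevalide flag is set and none of the three is off, otherwise SwitchOff.
; A never-reset DoOnce plays a Ding the first time it lights.
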(event `self.ReceiveBeginPlay`
  (`parent.ReceiveBeginPlay`)
  (bind _returnvalue (`GameplayStatics.GetActorOfClass` "/Game/Cabine/Blueprint/BP_LED_ATM.BP_LED_ATM_C"))
  (set `self.ATMLEDRef` _returnvalue)
  (bind _returnvalue_2 (`GameplayStatics.GetActorOfClass` "/Game/Cabine/Blueprint/BP_LED_Wheel.BP_LED_Wheel_C"))
  (set `self.WheelLEDRef` _returnvalue_2)
  (bind _returnvalue_3 (`GameplayStatics.GetActorOfClass` "/Game/Cabine/Blueprint/BP_LEDLevers.BP_LEDLevers_C"))
  (set `self.LeversLEDRef` _returnvalue_3)
  (bind _returnvalue_4 (`GameplayStatics.GetActorOfClass` "/Game/Cabine/Blueprint/BP_ControlPanel.BP_ControlPanel_C"))
  (set `self.Controlpanelref` _returnvalue_4))

(event `self.ReceiveTick`
  (params (DeltaSeconds :type "Float (single-precision)"))
  (`parent.ReceiveTick` DeltaSeconds)
  (if (`/Game/Cabine/Blueprint/BP_ControlPanel.Peutetrevalide` (`self.Controlpanelref`))
    (if (`/Game/Cabine/Blueprint/BP_LED.isOff` (`self.ATMLEDRef`))
      (`self.SwitchOff` :!label _label)
      (elif (`/Game/Cabine/Blueprint/BP_LED.isOff` (`self.WheelLEDRef`))
        (goto _label)
        (elif (`/Game/Cabine/Blueprint/BP_LED.isOff` (`self.LeversLEDRef`))
          (goto _label)
          (else
            (`self.SwitchOn`)
            (`/Engine/EditorBlueprintResources/StandardMacros.DoOnce` false
              (:`Completed`
                (`GameplayStatics.SpawnSound2D` "/Game/Others/Tests_Marie/Sons/ding.ding" 1.0 1.0 0.0 null)))))))
    (else
      (goto _label))))

(fn `SwitchOff`
  (`parent.SwitchOff`))

(fn `SwitchOn`
  (`parent.SwitchOn`))

(fn `UserConstructionScript`
  (`parent.UserConstructionScript`))