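; BP_LED is an LED actor that shows an on or off state by swapping the material on its LED component.
; It starts off at BeginPlay, and the SwitchOn and SwitchOff functions only set the IsOff flag.
; Tick reads that flag every frame and reapplies the matching on or off material instance, whether or not the state has changed.
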(event `self.ReceiveBeginPlay`
  (set `self.isOff` true))

(event `self.ReceiveTick`
  (params (DeltaSeconds :type "Float (single-precision)"))
  ; Set the material to turn the led on and off
  (if (`self.isOff`)
    (`PrimitiveComponent.SetMaterial` (`self.LED`) 0 "/Game/Materials/LED/M_LEDOff_Inst.M_LEDOff_Inst")
    (set `self.isOff` true)
    (else
      (`PrimitiveComponent.SetMaterial` (`self.LED`) 0 "/Game/Materials/LED/M_LEDOn_Inst.M_LEDOn_Inst")
      (set `self.isOff` false))))

(fn `SwitchOff`
  (set `self.isOff` true))

(fn `SwitchOn`
  (set `self.isOff` false))

(fn `UserConstructionScript`)