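; BP_ArmLever is a clickable lever that toggles back and forth between two angular positions.
; A click, ignored while the lever moves, flips the position index between 0 and 1 via a Reverse flag and derives start and end angles from it.
; The MoveLever timeline interpolates the Lever's pitch between them, then calls CallOnpositionUpdate when finished.
; The construction script sets Root's pitch to StartAngle.
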(event `self.ReceiveActorOnClicked`
  (params (ButtonPressed :type "Key Structure"))
  ; If the lever is already moving the player can't trigger it
  (if (not (`self.IsMoving`))
    (`self.ChangePositionIndex`)
    (set `self.IsMoving` true)
    (bind (_direction _lever) (`Timeline|MoveLever` :!via `PlayFromStart`)
      (:`Update`
        (`SceneComponent.K2_SetRelativeRotation` (`self.Lever`) (`KismetMathLibrary.MakeRotator` 0.0 (`KismetMathLibrary.Lerp` (`self.StartAngle`) (`self.EndAngle`) _lever)) false false))
      (:`Finished`
        (set `self.IsMoving` false)
        (`self.Onposition Update`)))))

(fn `ChangePositionIndex`
  ; Change the position and the number of the index
  (set `self.StartAngle` (* (`self.Angle`) (`self.PositionIndex`)))
  (if (`self.Reverse`)
    (bind _output_get (set `self.PositionIndex` (+ (`self.PositionIndex`) -1)))
    (if (== _output_get 0)
      (set `self.Reverse` false))
    (else
      (bind _output_get_2 (set `self.PositionIndex` (+ (`self.PositionIndex`) 1)))
      (if (== _output_get_2 1)
        (set `self.Reverse` true))))
  (set `self.EndAngle` (* (`self.Angle`) (`self.PositionIndex`))))

(fn `UserConstructionScript`
  (`SceneComponent.K2_SetRelativeRotation` (`self.root`) (`KismetMathLibrary.MakeRotator` 0.0 (`self.StartAngle`)) false false))